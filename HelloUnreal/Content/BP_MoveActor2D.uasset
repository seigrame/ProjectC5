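; BP_MoveActor2D is an actor that moves its MovingObject component back and forth along the relative X axis while IsPlay is true.
; Each Tick steps LocationX by a fixed amount and applies it as the relative location, flipping IsMoveRight once the value passes either bound.
; The step ignores delta time, so movement speed depends on frame rate.
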(event `self.ReceiveTick`
  (params (DeltaSeconds :type "Float (single-precision)"))
  (if (`self.isPlay`)
    (if (`self.isMoveRight`)
      ; 우로 이동
      (set `self.LocationX` (+ (`self.LocationX`) 10.0))
      (`SceneComponent.K2_SetRelativeLocation` (`self.MovingObject`) (`KismetMathLibrary.MakeVector` (`self.LocationX`)) false false)
      (if (> (`self.LocationX`) 500.0)
        (set `self.isMoveRight` false))
      (else
        ; 좌로 이동
        (set `self.LocationX` (+ (`self.LocationX`) -10.0))
        (`SceneComponent.K2_SetRelativeLocation` (`self.MovingObject`) (`KismetMathLibrary.MakeVector` (`self.LocationX`)) false false)
        (if (< (`self.LocationX`) 0.0)
          (set `self.isMoveRight` true))))))

(fn `UserConstructionScript`)