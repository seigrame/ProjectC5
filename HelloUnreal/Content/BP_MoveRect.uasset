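; BP_MoveRect is an actor that moves its static mesh along a square loop in the X-Z plane while IsPlay is true.
; Tick switches on a direction enum (Right, Up, Left, Down), stepping the mesh's relative location by a fixed amount each frame.
; Passing a bound advances the enum to the next side, forming a simple state machine.
; Movement ignores delta time, so speed depends on frame rate.
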(event `self.ReceiveTick`
  (params (DeltaSeconds :type "Float (single-precision)"))
  (if (`self.isPlay`)
    (switch `/Game/EN_MoveType` (`self.enumSwitch`)
      (:`NewEnumerator0`
        ; 우
        (set `self.LocationX` (+ (`self.LocationX`) 10.0))
        (`SceneComponent.K2_SetRelativeLocation` (`self.StaticMesh`) (`KismetMathLibrary.MakeVector` (`self.LocationX`) 0.0 (`self.LocationZ`)) false false)
        (if (> (`self.LocationX`) 500.0)
          (set `self.enumSwitch` "NewEnumerator1")))
      (:`NewEnumerator1`
        ; 상
        (set `self.LocationZ` (+ (`self.LocationZ`) 10.0))
        (`SceneComponent.K2_SetRelativeLocation` (`self.StaticMesh`) (`KismetMathLibrary.MakeVector` (`self.LocationX`) 0.0 (`self.LocationZ`)) false false)
        (if (> (`self.LocationZ`) 500.0)
          (set `self.enumSwitch` "NewEnumerator2")))
      (:`NewEnumerator2`
        ; 좌
        (set `self.LocationX` (+ (`self.LocationX`) -10.0))
        (`SceneComponent.K2_SetRelativeLocation` (`self.StaticMesh`) (`KismetMathLibrary.MakeVector` (`self.LocationX`) 0.0 (`self.LocationZ`)) false false)
        (if (< (`self.LocationX`) 0.0)
          (set `self.enumSwitch` "NewEnumerator3")))
      (:`NewEnumerator3`
        ; 하
        (set `self.LocationZ` (+ (`self.LocationZ`) -10.0))
        (`SceneComponent.K2_SetRelativeLocation` (`self.StaticMesh`) (`KismetMathLibrary.MakeVector` (`self.LocationX`) 0.0 (`self.LocationZ`)) false false)
        (if (< (`self.LocationZ`) 0.0)
          (set `self.enumSwitch` "NewEnumerator0"))))))

(fn `UserConstructionScript`)