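; BP_MoveStair is an actor that moves its static mesh around a closed, stair-shaped loop in the local X-Z plane.
; While IsPlay is true, Tick switches on an enum state and steps the mesh's relative location along one axis.
; Passing each leg's threshold advances the state through right, up, two left-then-down steps, then back to right.
; Steps are fixed per frame, so speed depends on frame rate.
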(event `self.ReceiveTick`
  (params (DeltaSeconds :type "Float (single-precision)"))
  (if (`self.isPlay`)
    (switch `/Game/EN_MoveStair` (`self.enumSwitch`)
      (:`NewEnumerator0`
        ; 우
        (set `self.LocationX` (+ (`self.LocationX`) 10.0))
        (`SceneComponent.K2_SetRelativeLocation` (`self.StaticMesh`) (`KismetMathLibrary.MakeVector` (`self.LocationX`) 0.0 (`self.LocationZ`)) false false)
        (if (> (`self.LocationX`) 500.0)
          (set `self.enumSwitch` "NewEnumerator1")))
      (:`NewEnumerator1`
        ; 상
        (set `self.LocationZ` (+ (`self.LocationZ`) 10.0))
        (`SceneComponent.K2_SetRelativeLocation` (`self.StaticMesh`) (`KismetMathLibrary.MakeVector` (`self.LocationX`) 0.0 (`self.LocationZ`)) false false)
        (if (> (`self.LocationZ`) 500.0)
          (set `self.enumSwitch` "NewEnumerator2")))
      (:`NewEnumerator2`
        ; 좌1
        (set `self.LocationX` (+ (`self.LocationX`) -10.0))
        (`SceneComponent.K2_SetRelativeLocation` (`self.StaticMesh`) (`KismetMathLibrary.MakeVector` (`self.LocationX`) 0.0 (`self.LocationZ`)) false false)
        (if (< (`self.LocationX`) 250.0)
          (set `self.enumSwitch` "NewEnumerator3")))
      (:`NewEnumerator3`
        ; 하1
        (set `self.LocationZ` (+ (`self.LocationZ`) -10.0))
        (`SceneComponent.K2_SetRelativeLocation` (`self.StaticMesh`) (`KismetMathLibrary.MakeVector` (`self.LocationX`) 0.0 (`self.LocationZ`)) false false)
        (if (< (`self.LocationZ`) 250.0)
          (set `self.enumSwitch` "NewEnumerator4")))
      (:`NewEnumerator4`
        ; 좌2
        (set `self.LocationX` (+ (`self.LocationX`) -10.0))
        (`SceneComponent.K2_SetRelativeLocation` (`self.StaticMesh`) (`KismetMathLibrary.MakeVector` (`self.LocationX`) 0.0 (`self.LocationZ`)) false false)
        (if (< (`self.LocationX`) 0.0)
          (set `self.enumSwitch` "NewEnumerator5")))
      (:`NewEnumerator5`
        ; 하2
        (set `self.LocationZ` (+ (`self.LocationZ`) -10.0))
        (`SceneComponent.K2_SetRelativeLocation` (`self.StaticMesh`) (`KismetMathLibrary.MakeVector` (`self.LocationX`) 0.0 (`self.LocationZ`)) false false)
        (if (< (`self.LocationZ`) 0.0)
          (set `self.enumSwitch` "NewEnumerator0"))))))

(fn `UserConstructionScript`)