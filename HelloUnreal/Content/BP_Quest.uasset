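; BP_Quest is a Blueprint that prints the pieces of a comma-separated string variable, Strings, as debug messages.
; While Strings is longer than three characters, each Tick prints the text before the first comma and keeps the remainder, consuming one piece per frame.
; An unconnected, hand-unrolled chain of the same split-and-print steps never runs, and BeginPlay and the construction script are empty.
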(event `self.ReceiveBeginPlay`)

(event `self.ReceiveTick`
  (params (DeltaSeconds :type "Float (single-precision)"))
  (bind (_lefts _rights) (`KismetStringLibrary.Split` (`self.Strings`) ","))
  (if (> (`KismetStringLibrary.Len` (`self.Strings`)) 3)
    (`KismetSystemLibrary.PrintString` _lefts true true (struct :`G` 0.66 :`B` 1.0 :`A` 1.0) 10.0)
    (set `self.Strings` _rights)))

(fn `UserConstructionScript`)