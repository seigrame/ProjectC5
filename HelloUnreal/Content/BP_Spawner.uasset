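; BP_Spawner is an actor that spawns a batch of BP_Ball actors at random points inside its collision box.
; The BoolSpawn event loops until Count reaches five, placing each ball within the box's scaled extent using the spawner's rotation.
; It increments BallCount per spawn and prints each index and the final tally.
; Count is never reset here, so later calls spawn nothing once the limit is reached.
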(event `BoolSpawn`
  (bind _count (`self.count`))
  (while (< _count 5)
    (`/Engine/EditorBlueprintResources/StandardMacros.IncrementInt` (`self.count`)
      (:`  `
        (`/Engine/EditorBlueprintResources/StandardMacros.IncrementInt` (`self.ballCount`)
          (:`  `
            (`KismetSystemLibrary.PrintString` (`KismetStringLibrary.Concat_StrStr` "index :" (`KismetStringLibrary.Conv_IntToString` _count)))
            (`|SpawnActorFromClass` "/Game/BP_Ball.BP_Ball_C" (`KismetMathLibrary.MakeTransform` (`KismetMathLibrary.RandomPointInBoundingBox` (`self.K2_GetActorLocation`) (`BoxComponent.GetScaledBoxExtent` (`self.BoxCollision`))) (`self.K2_GetActorRotation`)) "Undefined" "MultiplyWithRoot" null null))))))
  (bind _output_get (set `self.ballCount` (`self.ballCount`)))
  (`KismetSystemLibrary.PrintString` (`KismetStringLibrary.Conv_IntToString` _output_get) true true (struct :`G` 0.66 :`B` 1.0 :`A` 1.0) 60.0))

(fn `UserConstructionScript`)