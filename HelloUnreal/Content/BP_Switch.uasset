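; BP_Switch is an overlap switch that pauses linked moving actors and triggers a ball spawner.
; When its StaticMesh begins an overlap, it sets IsPlay false on MoveActor2D, MoveRect and MoveStair, then calls BoolSpawn and resets the Spawner's Count if BallCount is under a cap.
; When the overlap ends, it sets IsPlay true on those movers again.
; Overlap event-log prints remain in the graph but never run.
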(event `self.StaticMesh.OnComponentBeginOverlap`
  (params (OverlappedComponent :type "PrimitiveComponent Object Reference") (OtherActor :type "Actor Object Reference") (OtherComp :type "PrimitiveComponent Object Reference") (OtherBodyIndex :type Integer) (bFromSweep :type Boolean) (SweepResult :type "HitResult Structure (by ref)"))
  (bind _moverect (`self.MoveRect`))
  (bind _movestair (`self.MoveStair`))
  (bind _moveactor2d (`self.MoveActor2D`))
  (bind _ballcount (`/Game/BP_Spawner.ballCount` (`self.Spawner`)))
  (`|ExecutionSequence`
    (:`then_0`
      (`/Engine/EditorBlueprintResources/StandardMacros.IsValid` _moveactor2d
        (:`Is Valid`
          (set `/Game/BP_MoveActor2D.isPlay` false _moveactor2d))
        (:`Is Not Valid`
          (`KismetSystemLibrary.PrintString` "isNullPtr" true true (struct :`R` 1.0 :`A` 1.0)))))
    (:`then_1`
      (`/Engine/EditorBlueprintResources/StandardMacros.IsValid` _moverect
        (:`Is Valid`
          (set `/Game/BP_MoveRect.isPlay` false _moverect))
        (:`Is Not Valid`
          (`KismetSystemLibrary.PrintString` "isNullPtr" true true (struct :`R` 1.0 :`A` 1.0)))))
    (:`then_2`
      (`/Engine/EditorBlueprintResources/StandardMacros.IsValid` _movestair
        (:`Is Valid`
          (set `/Game/BP_MoveStair.isPlay` false _movestair))
        (:`Is Not Valid`
          (`KismetSystemLibrary.PrintString` "isNullPtr" true true (struct :`R` 1.0 :`A` 1.0)))))
    (:`then_3`
      (`KismetSystemLibrary.PrintString` (`KismetStringLibrary.Conv_IntToString` _ballcount))
      (if (< _ballcount 20)
        (`/Game/BP_Spawner.BoolSpawn` (`self.Spawner`))
        (set `/Game/BP_Spawner.count` 0 (`self.Spawner`))))))

(event `self.StaticMesh.OnComponentEndOverlap`
  (params (OverlappedComponent :type "PrimitiveComponent Object Reference") (OtherActor :type "Actor Object Reference") (OtherComp :type "PrimitiveComponent Object Reference") (OtherBodyIndex :type Integer))
  (bind _moveactor2d (`self.MoveActor2D`))
  (bind _moverect (`self.MoveRect`))
  (bind _movestair (`self.MoveStair`))
  (`|ExecutionSequence`
    (:`then_0`
      (`/Engine/EditorBlueprintResources/StandardMacros.IsValid` _moveactor2d
        (:`Is Valid`
          (set `/Game/BP_MoveActor2D.isPlay` true _moveactor2d))))
    (:`then_1`
      (`/Engine/EditorBlueprintResources/StandardMacros.IsValid` _moverect
        (:`Is Valid`
          (set `/Game/BP_MoveRect.isPlay` true _moverect))))
    (:`then_2`
      (`/Engine/EditorBlueprintResources/StandardMacros.IsValid` _movestair
        (:`Is Valid`
          (set `/Game/BP_MoveStair.isPlay` true _movestair))))))

(fn `UserConstructionScript`)