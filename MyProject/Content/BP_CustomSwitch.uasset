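; BP_CustomSwitch is an overlap switch that pauses or resumes linked rect and stair objects and triggers a spawner.
; Beginning an overlap with its Cube component clears IsPlay on RectObj and StairObj, then calls BoolSpawn on Spawner.
; Ending the overlap sets IsPlay back to true on both objects, without calling the spawner.
; Both objects are validity-checked with a printed fallback, while Spawner is unchecked and overlapping actors are unfiltered.
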(event `self.Cube.OnComponentBeginOverlap`
  (params (OverlappedComponent :type "PrimitiveComponent Object Reference") (OtherActor :type "Actor Object Reference") (OtherComp :type "PrimitiveComponent Object Reference") (OtherBodyIndex :type Integer) (bFromSweep :type Boolean) (SweepResult :type "HitResult Structure (by ref)"))
  (bind _rectobj (`self.RectObj`))
  (bind _stairobj (`self.StairObj`))
  (`|ExecutionSequence`
    (:`then_0`
      (`/Engine/EditorBlueprintResources/StandardMacros.IsValid` _rectobj
        (:`Is Valid`
          (set `/Game/BP_Rect.isPlay` false _rectobj))
        (:`Is Not Valid`
          (`KismetSystemLibrary.PrintString` "Null" true true (struct :`R` 1.0 :`A` 1.0)))))
    (:`then_1`
      (`/Engine/EditorBlueprintResources/StandardMacros.IsValid` _stairobj
        (:`Is Valid`
          (set `/Game/BP_Stair.isPlay` false _stairobj))
        (:`Is Not Valid`
          (`KismetSystemLibrary.PrintString` "Null" true true (struct :`R` 1.0 :`A` 1.0)))))
    (:`then_2`
      (`/Game/BP_SpawnArea.BoolSpawn` (`self.Spawner`)))))

(event `self.Cube.OnComponentEndOverlap`
  (params (OverlappedComponent :type "PrimitiveComponent Object Reference") (OtherActor :type "Actor Object Reference") (OtherComp :type "PrimitiveComponent Object Reference") (OtherBodyIndex :type Integer))
  (bind _rectobj (`self.RectObj`))
  (bind _stairobj (`self.StairObj`))
  (`|ExecutionSequence`
    (:`then_0`
      (`/Engine/EditorBlueprintResources/StandardMacros.IsValid` _rectobj
        (:`Is Valid`
          (set `/Game/BP_Rect.isPlay` true _rectobj))
        (:`Is Not Valid`
          (`KismetSystemLibrary.PrintString` "Null" true true (struct :`R` 1.0 :`A` 1.0)))))
    (:`then_1`
      (`/Engine/EditorBlueprintResources/StandardMacros.IsValid` _stairobj
        (:`Is Valid`
          (set `/Game/BP_Stair.isPlay` true _stairobj))
        (:`Is Not Valid`
          (`KismetSystemLibrary.PrintString` "Null" true true (struct :`R` 1.0 :`A` 1.0)))))))

(fn `UserConstructionScript`)