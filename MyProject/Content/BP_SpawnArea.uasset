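; BP_SpawnArea is a spawner actor that fills a box-shaped area with BP_Ball actors.
; Its BoolSpawn event loops until Count reaches five, spawning a ball at a random point inside the BoxCollision bounds with the spawner's rotation.
; Count is never reset here, so later calls spawn nothing once that limit is reached.
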(event `BoolSpawn`
  (while (< (`self.Count`) 5)
    (`/Engine/EditorBlueprintResources/StandardMacros.IncrementInt` (`self.Count`)
      (:`  `
        (`|SpawnActorFromClass` "/Game/BP_Ball.BP_Ball_C" (`KismetMathLibrary.MakeTransform` (`KismetMathLibrary.RandomPointInBoundingBox` (`self.K2_GetActorLocation`) (`BoxComponent.GetScaledBoxExtent` (`self.BoxCollision`))) (`self.K2_GetActorRotation`)) "Undefined" "MultiplyWithRoot" null null)))))

(fn `UserConstructionScript`)