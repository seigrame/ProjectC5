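; BP_Stair is an actor that moves a Cube component around a closed, stair-shaped path in its local X-Z plane.
; While IsPlay is true, Tick switches on the SwitchRect state and steps the cube's relative location by a fixed amount each frame, independent of delta time.
; Crossing each segment's threshold advances the state through right, up, and two left-down steps, then loops.
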(event `self.ReceiveTick`
  (params (DeltaSeconds :type "Float (single-precision)"))
  (if (`self.isPlay`)
    (switch `/Game/EN_Stair` (`self.SwitchRect`)
      (:`NewEnumerator0`
        (set `self.LocationX` (+ (`self.LocationX`) 10.0))
        (`SceneComponent.K2_SetRelativeLocation` (`self.Cube`) (`KismetMathLibrary.MakeVector` (`self.LocationX`) 0.0 (`self.LocationZ`)) false false)
        (if (> (`self.LocationX`) 500.0)
          (set `self.SwitchRect` "NewEnumerator1")))
      (:`NewEnumerator1`
        (set `self.LocationZ` (+ (`self.LocationZ`) 10.0))
        (`SceneComponent.K2_SetRelativeLocation` (`self.Cube`) (`KismetMathLibrary.MakeVector` (`self.LocationX`) 0.0 (`self.LocationZ`)) false false)
        (if (> (`self.LocationZ`) 500.0)
          (set `self.SwitchRect` "NewEnumerator2")))
      (:`NewEnumerator2`
        (set `self.LocationX` (+ (`self.LocationX`) -10.0))
        (`SceneComponent.K2_SetRelativeLocation` (`self.Cube`) (`KismetMathLibrary.MakeVector` (`self.LocationX`) 0.0 (`self.LocationZ`)) false false)
        (if (< (`self.LocationX`) 250.0)
          (set `self.SwitchRect` "NewEnumerator3")))
      (:`NewEnumerator3`
        (set `self.LocationZ` (+ (`self.LocationZ`) -10.0))
        (`SceneComponent.K2_SetRelativeLocation` (`self.Cube`) (`KismetMathLibrary.MakeVector` (`self.LocationX`) 0.0 (`self.LocationZ`)) false false)
        (if (< (`self.LocationZ`) 250.0)
          (set `self.SwitchRect` "NewEnumerator4")))
      (:`NewEnumerator4`
        (set `self.LocationX` (+ (`self.LocationX`) -10.0))
        (`SceneComponent.K2_SetRelativeLocation` (`self.Cube`) (`KismetMathLibrary.MakeVector` (`self.LocationX`) 0.0 (`self.LocationZ`)) false false)
        (if (< (`self.LocationX`) 0.0)
          (set `self.SwitchRect` "NewEnumerator5")))
      (:`NewEnumerator5`
        (set `self.LocationZ` (+ (`self.LocationZ`) -10.0))
        (`SceneComponent.K2_SetRelativeLocation` (`self.Cube`) (`KismetMathLibrary.MakeVector` (`self.LocationX`) 0.0 (`self.LocationZ`)) false false)
        (if (< (`self.LocationZ`) 0.0)
          (set `self.SwitchRect` "NewEnumerator0"))))))

(fn `UserConstructionScript`)